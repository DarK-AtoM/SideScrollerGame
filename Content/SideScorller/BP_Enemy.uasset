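; Side-scroller enemy that walks forward and turns around when it meets a wall.
; Each Tick adds forward movement input, while a short line trace from Arrow1 detects walls, with a DoOnce limiting the flip to once per detection.
; Body overlap damages the side-scroll character.
; Head overlap awards it score and, if it is tagged Player, destroys the enemy with a steam effect.
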(event `self.Body.OnComponentBeginOverlap`
  (params (OverlappedComponent :type "PrimitiveComponent Object Reference") (OtherActor :type "Actor Object Reference") (OtherComp :type "PrimitiveComponent Object Reference") (OtherBodyIndex :type Integer) (bFromSweep :type Boolean) (SweepResult :type "HitResult Structure (by ref)"))
  (bind _asbp_side_scroll_character (cast `/Game/SideScorller/BP_SideScrollCharacter` OtherActor))
  (`/Game/SideScorller/BP_SideScrollCharacter.TakeDamage` _asbp_side_scroll_character))

(event `self.Head.OnComponentBeginOverlap`
  (params (OverlappedComponent :type "PrimitiveComponent Object Reference") (OtherActor :type "Actor Object Reference") (OtherComp :type "PrimitiveComponent Object Reference") (OtherBodyIndex :type Integer) (bFromSweep :type Boolean) (SweepResult :type "HitResult Structure (by ref)"))
  (bind _asbp_side_scroll_character (cast `/Game/SideScorller/BP_SideScrollCharacter` OtherActor))
  (set `/Game/SideScorller/BP_SideScrollCharacter.Score` (+ (`/Game/SideScorller/BP_SideScrollCharacter.Score` _asbp_side_scroll_character) 20) _asbp_side_scroll_character)
  (if (`self.ActorHasTag` OtherActor "Player")
    (`GameplayStatics.SpawnEmitterAtLocation` "/Game/StarterContent/Particles/P_Steam_Lit.P_Steam_Lit" (`self.K2_GetActorLocation`))
    (`self.K2_DestroyActor`)))

(event `self.ReceiveTick`
  (params (DeltaSeconds :type "Float (single-precision)"))
  (`|ExecutionSequence`
    (:`then_0`
      (bind _newparameter (`self.LineTraceWall`))
      (if _newparameter
        (`/Engine/EditorBlueprintResources/StandardMacros.DoOnce` false :!label _label
          (:`Completed`
            (`MovementComponent.StopMovementImmediately` (`self.CharacterMovement`))
            (`self.K2_AddActorWorldRotation` (struct :`Yaw` 180.0))))
        (else
          (goto _label :!via `Reset`))))
    (:`then_1`
      (`self.AddMovementInput` (`KismetMathLibrary.GetForwardVector` (`self.K2_GetActorRotation`))))))

(fn `LineTraceWall`
  (returns (NewParameter :type Boolean))
  (bind _arrow1 (`self.Arrow1`))
  (bind _returnvalue (`SceneComponent.K2_GetComponentLocation` _arrow1))
  (bind (_outhit _returnvalue_2) (`KismetSystemLibrary.LineTraceSingle` _returnvalue (+ _returnvalue (* (`KismetMathLibrary.GetForwardVector` (`SceneComponent.K2_GetComponentRotation` _arrow1)) 130.0)) "TraceTypeQuery1"))
  (return _returnvalue_2))

(fn `UserConstructionScript`)